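; Enemy that wanders, chases the first-person player on sight or sound, and destroys them within attack range.
; Wandering repeats random reachable moves after each success; PawnSensing starts a chase via AI MoveTo.
; A looping timer polls the player's light during the chase and reissues the move on change, using a much larger acceptance radius when lit.
; Tick handles the kill, with a placeholder for an ending screen.
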(event `self.ReceiveBeginPlay`
  (`|AIMoveTo` self (`NavigationSystemV1.K2_GetRandomReachablePointInRadius` (`self.K2_GetActorLocation`) 1000.0 null null) null :!label _label
    (:`OnSuccess`
      (`KismetSystemLibrary.Delay` 1.0)
      (goto _label))))

(event `self.PawnSensing.OnSeePawn`
  (params (Pawn :type "Pawn Object Reference"))
  (set `self.target` Pawn)
  (if (not (`self.IsSeeingPlayer?`)) :!label _label_2
    (set `self.IsSeeingPlayer?` true)
    (`self.FollowPlayer` (`self.target`))))

(event `self.PawnSensing.OnHearNoise`
  (params (Instigator :type "Pawn Object Reference") (Location :type "Vector Structure (by ref)") (Volume :type "Float (single-precision)"))
  (set `self.target` Instigator)
  (goto _label_2))

(event `self.ReceiveTick`
  (params (DeltaSeconds :type "Float (single-precision)"))
  (bind _player (`self.Player`)
    (:`then`
      (if (<= (`self.GetDistanceTo` _player) (`self.AttackRanger`))
        ;[1 1 1] Tu jakas logika ending screen xd
        (`self.K2_DestroyActor` (`self.Player`))))
    (:`else`)))

(event `FollowPlayer`
  (params (Pawn :type "Pawn Object Reference"))
  (bind _asbp_first_person_character (cast `/Game/FirstPerson/Blueprints/BP_FirstPersonCharacter` Pawn))
  (bind _output_get (set `self.Player` _asbp_first_person_character))
  (bind _returnvalue (`KismetSystemLibrary.K2_SetTimerDelegate` (delegate `CheckLight`) 0.1 true true))
  (set `self.Check light Timer` _returnvalue)
  (`self.UpdateLocation` (`/Game/FirstPerson/Blueprints/BP_FirstPersonCharacter.IsLightON?` _output_get)))

(event `UpdateLocation`
  (params (Condition :type Boolean))
  (if Condition
    (set `self.DefaultRadius` 500.0)
    (else
      (set `self.DefaultRadius` 50.0)))
  (bind _player (`self.Player`)
    (:`then`
      (`|AIMoveTo` self (0.0 0.0 0.0) _player (`self.DefaultRadius`)
        (:`OnSuccess`
          _)
        (:`OnFail`
          _)))
    (:`else`
      _))
  (set `self.IsSeeingPlayer?` false)
  (`KismetSystemLibrary.K2_ClearAndInvalidateTimerHandle` (`self.Check light Timer`)))

(event `CheckLight`
  (bind _player (`self.Player`)
    (:`then`
      (bind _islighton_ (`/Game/FirstPerson/Blueprints/BP_FirstPersonCharacter.IsLightON?` _player))
      (if (!= _islighton_ (`self.Last Value`))
        (set `self.Last Value` _islighton_)
        (`self.UpdateLocation` _islighton_)))
    (:`else`
      (set `self.IsSeeingPlayer?` false)
      (`KismetSystemLibrary.K2_ClearAndInvalidateTimerHandle` (`self.Check light Timer`)))))

(fn `UserConstructionScript`)