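; BP_Crystal is a crystal actor that highlights its static mesh through Custom Depth rendering while the player is searching.
; A looping timer started on BeginPlay polls the IsPlayerSearching flag and turns the mesh's custom depth on or off, avoiding Tick.
; The flag is not set within this Blueprint, and the separate CustomDepthON function and CustomDepthOFF event are empty stubs.
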(event `self.ReceiveBeginPlay`
  (`KismetSystemLibrary.K2_SetTimerDelegate` (delegate `DEPTH`) 0.1 true))

(event `DEPTH`
  (if (`self.IsPlayerSearching?`)
    (`self.CrystalDepthON`)
    (else
      (`self.CrystalDepthOFF`))))

(event `CrystalDepthON`
  (`PrimitiveComponent.SetRenderCustomDepth` (`self.StaticMesh`) true))

(event `CrystalDepthOFF`
  (`PrimitiveComponent.SetRenderCustomDepth` (`self.StaticMesh`) false))

(event `CustomDepthOFF`)

(fn `CustomDepthON`)

(fn `UserConstructionScript`)