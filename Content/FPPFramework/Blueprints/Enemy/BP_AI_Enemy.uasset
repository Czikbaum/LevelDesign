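; Modular melee enemy character that senses the player, turns toward and chases them, and forgets them after a delay once sight or stimulus is lost.
; Tick picks between chase, a cooldown-gated launch dash that triggers player slow motion when it ends, and random montage-section attacks.
; Hand-socket sphere traces apply damage.
; Damage triggers throttled hit reactions; death plays a montage and detaches a random leader-pose body part as an impulsed physics object.
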(event `self.ReceiveBeginPlay`
  (set `self.ModularMeshes` (`|MakeArray` (`self.R_Leg`) (`self.R_Arm`) (`self.L_Leg`) (`self.L_Arm`) (`self.Head`))))

(event `self.AIPerception.OnTargetPerceptionUpdated`
  (params (Actor :type "Actor Object Reference") (Stimulus :type "AIStimulus Structure"))
  ;[0 0 0] On Perception Updated
  (if (`.bSuccessfullySensed` (break `AIStimulus` Stimulus))
    (bind _asbp_fpp_character (cast `/Game/FPPFramework/Blueprints/BP_FPP_Character` Actor)
      (:`then`
        (`KismetSystemLibrary.K2_ClearAndInvalidateTimerHandle` (`self.TargetForgotHandle`))
        (set `self.TargetActor` _asbp_fpp_character))
      (:`CastFailed`
        (`KismetSystemLibrary.K2_ClearAndInvalidateTimerHandle` (`self.TargetForgotHandle`) :!label _label)
        (bind _returnvalue (`KismetSystemLibrary.K2_SetTimer` null "ForgetTarget" (`self.TargetForgotDelay`)))
        (set `self.TargetForgotHandle` _returnvalue)))
    (else
      (goto _label))))

(event `self.ReceiveTick`
  (params (DeltaSeconds :type "Float (single-precision)"))
  (bind _returnvalue (`self.GetDistanceTo` (`self.TargetActor`)))
  ;[0 0 0] AI Logic
  (if (!= (`self.TargetActor`) null)
    (`self.ComputeAIRotation` DeltaSeconds)
    (if (and (not (`self.bIsReactingToHit`)) (not (`self.bIsAttacking`)))
      (if (> _returnvalue (`self.AttackRange`))
        (if (and (< _returnvalue (`self.DashRange`)) (`self.bCanDash`))
          (`self.PerformDash`)
          (else
            (`self.ChasePlayer`)))
        (elif (`self.bCanAttack`)
          (`self.PerformMeleeAttack`))))))

(event `ChasePlayer`
  ;[0 0 0] Chase Player (move to target)
  (bind _targetactor (`self.TargetActor`)
    (:`then`
      (`|AIMoveTo` self (0.0 0.0 0.0) _targetactor (* (`self.AttackRange`) 0.8)))
    (:`else`)))

(event `PlayMontage`
  (params (MontageToPlay :type "AnimMontage Object Reference"))
  ;[0 0 0] Play Montage
  (`|PlayMontage` (`self.Mesh`) MontageToPlay))

(event `self.ReceiveAnyDamage`
  (params (Damage :type "Float (single-precision)") (DamageType :type "DamageType Object Reference") (InstigatedBy :type "Controller Object Reference") (DamageCauser :type "Actor Object Reference"))
  (bind _sfx (`self.GetRandomSFX` "NewEnumerator1"))
  ;[0 0 0] Taken damage
  (set `self.Health` (`KismetMathLibrary.FClamp` (- (`self.Health`) Damage) 0.0 100.0))
  (if (<= (`self.Health`) 0.0)
    (`KismetSystemLibrary.Delay` 0.1)
    (`self.OnDied`)
    (elif (`self.bCanReactToHit`)
      (set `self.bCanReactToHit` false)
      (`self.OnHitReaction`)
      (`/Engine/EditorBlueprintResources/StandardMacros.IsValid` _sfx
        (:`Is Valid`
          (`GameplayStatics.PlaySoundAtLocation` _sfx (`self.K2_GetActorLocation`) (struct) 1.0 1.0 0.0 null null null null))))))

(fn `ComputeAIRotation`
  (params (DeltaTime :type "Float (single-precision)"))
  (`self.K2_SetActorRotation` (`KismetMathLibrary.RInterpTo_Constant` (`self.K2_GetActorRotation`) (`KismetMathLibrary.FindLookAtRotation` (`self.K2_GetActorLocation`) (`self.K2_GetActorLocation` (`self.TargetActor`))) DeltaTime 250.0)))

(fn `DoDamageTrace`
  (params (Source :type "/Game/FPPFramework/Data/AI/E_DamageTraceSource Enum" :default "NewEnumerator0"))
  (locals (InSocket :type Name :default "None"))
  (bind _returnvalue (`SceneComponent.GetSocketLocation` (`self.Mesh`) (`local.InSocket`)))
  (switch `/Game/FPPFramework/Data/AI/E_DamageTraceSource` Source
    (:`NewEnumerator0`
      (set `local.InSocket` "LeftHand"))
    (:`NewEnumerator1`
      (set `local.InSocket` "RightHand")))
  (bind (_outhit _returnvalue_2) (`KismetSystemLibrary.SphereTraceSingle` :`Start` _returnvalue :`End` _returnvalue :`Radius` 25.0 :`TraceChannel` "TraceTypeQuery4" :`DrawDebugType` "ForDuration"))
  (if _returnvalue_2
    (`GameplayStatics.ApplyDamage` (`.HitActor` (`GameplayStatics.BreakHitResult` _outhit)) (`self.Damage`))))

(fn `EndAttack`
  (bind _attackmontage (`self.AttackMontage`)
    (:`then`
      (`AnimInstance.Montage_Stop` (`SkeletalMeshComponent.GetAnimInstance` (`self.Mesh`)) 0.25 _attackmontage))
    (:`else`
      _))
  (set `self.bIsAttacking` false))

(fn `EndDash`
  (`Controller.StopMovement` (`AIBlueprintHelperLibrary.GetAIController` self))
  (set `self.bIsAttacking` false)
  (bind _asbp_fpp_character (cast `/Game/FPPFramework/Blueprints/BP_FPP_Character` (`self.TargetActor`)))
  (`/Game/FPPFramework/Blueprints/BP_FPP_Character.TriggerSlowMotion` _asbp_fpp_character))

(fn `ForgetTarget`
  (set `self.TargetActor` null))

(fn `GetRandomSFX`
  (params (InType :type "/Game/FPPFramework/Data/SFX/E_EnemySFXType Enum" :default "NewEnumerator0"))
  (returns (SFX :type "SoundBase Object Reference"))
  (bind (_attacksfx _damagedsfx _diedsfx) (break `/Game/FPPFramework/Data/SFX/ST_EnemySFXData` (`self.SFXData`)))
  (bind _outitem (`KismetArrayLibrary.Array_Random` _diedsfx))
  (bind _outitem_2 (`KismetArrayLibrary.Array_Random` _attacksfx))
  (bind _outitem_3 (`KismetArrayLibrary.Array_Random` _damagedsfx))
  (switch `/Game/FPPFramework/Data/SFX/E_EnemySFXType` InType
    (:`NewEnumerator0`
      (`/Engine/EditorBlueprintResources/StandardMacros.IsValid` _outitem_2
        (:`Is Valid`
          (return _outitem_2))
        (:`Is Not Valid`
          _)))
    (:`NewEnumerator1`
      (`/Engine/EditorBlueprintResources/StandardMacros.IsValid` _outitem_3
        (:`Is Valid`
          (return _outitem_3))
        (:`Is Not Valid`
          _)))
    (:`NewEnumerator2`
      (`/Engine/EditorBlueprintResources/StandardMacros.IsValid` _outitem
        (:`Is Valid`
          (return _outitem))
        (:`Is Not Valid`
          _))))
  (return null))

(fn `OnDied`
  (locals (SectionName :type Name) (CachedPart :type "SkeletalMeshComponent Object Reference"))
  (bind _sfx (`self.GetRandomSFX` "NewEnumerator2"))
  (bind _cachedpart (`local.CachedPart`))
  (bind _outitem (`KismetArrayLibrary.Array_Random` (`self.ModularMeshes`)))
  (`/Engine/EditorBlueprintResources/StandardMacros.IsValid` _sfx
    (:`Is Valid`
      (`GameplayStatics.PlaySoundAtLocation` _sfx (`self.K2_GetActorLocation`) (struct) 1.0 1.0 0.0 null null null null))
    (:`Is Not Valid`
      _))
  (`Controller.StopMovement` (`AIBlueprintHelperLibrary.GetAIController` self))
  (`self.SetActorTickEnabled` false)
  (`PrimitiveComponent.SetCollisionResponseToChannel` (`self.Mesh`) "ECC_GameTraceChannel5" "ECR_Ignore")
  (`PrimitiveComponent.SetCollisionResponseToChannel` (`self.R_Arm`) "ECC_GameTraceChannel5" "ECR_Ignore")
  (`PrimitiveComponent.SetCollisionResponseToChannel` (`self.Lower_Torso`) "ECC_GameTraceChannel5" "ECR_Ignore")
  (`PrimitiveComponent.SetCollisionResponseToChannel` (`self.L_Leg`) "ECC_GameTraceChannel5" "ECR_Ignore")
  (`PrimitiveComponent.SetCollisionResponseToChannel` (`self.L_Arm`) "ECC_GameTraceChannel5" "ECR_Ignore")
  (`PrimitiveComponent.SetCollisionResponseToChannel` (`self.Head`) "ECC_GameTraceChannel5" "ECR_Ignore")
  (`PrimitiveComponent.SetCollisionResponseToChannel` (`self.R_Leg`) "ECC_GameTraceChannel5" "ECR_Ignore")
  (`PrimitiveComponent.SetCollisionResponseToChannel` (`self.CapsuleComponent`) "ECC_Pawn" "ECR_Ignore")
  (`self.PlayMontage` "/Game/FPPFramework/Character/Enemy/AM_Monster_Death.AM_Monster_Death")
  (`/Engine/EditorBlueprintResources/StandardMacros.IsValid` _outitem
    (:`Is Valid`
      (set `local.CachedPart` _outitem)
      (`SkinnedMeshComponent.SetLeaderPoseComponent` _cachedpart null false false)
      (`PrimitiveComponent.SetCollisionProfileName` _cachedpart "Ragdoll" true)
      (`PrimitiveComponent.SetSimulatePhysics` _cachedpart true)
      (`SceneComponent.K2_DetachFromComponent` _cachedpart "KeepWorld" "KeepWorld" "KeepWorld" true)
      (`PrimitiveComponent.AddImpulse` _cachedpart (* (* (* (`self.GetActorForwardVector`) -1) (`PrimitiveComponent.GetMass` _cachedpart)) 100.0) "None" true))))

(fn `OnHitReaction`
  (locals (SectionName :type Name))
  (bind _hitreactionmontage (`self.HitReactionMontage`))
  (set `self.bIsReactingToHit` true)
  (`Controller.StopMovement` (`AIBlueprintHelperLibrary.GetAIController` self))
  (set `local.SectionName` (`KismetStringLibrary.Conv_StringToName` (`KismetTextLibrary.Conv_TextToString` (`|FormatText` "HitReaction_{Index}" (`KismetMathLibrary.RandomIntegerInRange` 1 7)))))
  (`self.PlayMontage` _hitreactionmontage)
  (`AnimInstance.Montage_JumpToSection` (`SkeletalMeshComponent.GetAnimInstance` (`self.Mesh`)) (`local.SectionName`) _hitreactionmontage))

(fn `OnHitReactionEnded`
  (set `self.bIsReactingToHit` false)
  (`KismetSystemLibrary.K2_SetTimer` null "ResetHitReact" (`self.HitReactionCooldown`)))

(fn `PerformDash`
  (locals (Direction :type "Vector Structure"))
  (set `self.bIsAttacking` true)
  (set `self.bCanDash` false)
  (bind _targetactor (`self.TargetActor`)
    (:`then`
      (`Controller.StopMovement` (`AIBlueprintHelperLibrary.GetAIController` self))
      (set `local.Direction` (`KismetMathLibrary.Normal` (- (`self.K2_GetActorLocation` _targetactor) (`self.K2_GetActorLocation`))))
      (`self.LaunchCharacter` (* (`self.DashSpeed`) (`local.Direction`))))
    (:`else`
      _))
  (`KismetSystemLibrary.K2_SetTimer` null "EndDash" (`self.DashDuration`))
  (`KismetSystemLibrary.K2_SetTimer` null "ResetDashCooldown" (`self.DashCooldown`)))

(fn `PerformMeleeAttack`
  (locals (RandomAnimIndex :type Integer) (SectionName :type Name))
  (bind _sfx (`self.GetRandomSFX` "NewEnumerator0"))
  (set `self.bIsAttacking` true)
  (set `self.bCanAttack` false)
  (set `local.RandomAnimIndex` (`KismetMathLibrary.RandomIntegerInRange` 1 (`self.NumSections`)))
  (set `local.SectionName` (`KismetStringLibrary.Conv_StringToName` (`KismetTextLibrary.Conv_TextToString` (`|FormatText` "Attack_{Index}" (`local.RandomAnimIndex`)))))
  (bind _attackmontage (`self.AttackMontage`)
    (:`then`
      (`self.PlayMontage` _attackmontage)
      (`AnimInstance.Montage_JumpToSection` (`SkeletalMeshComponent.GetAnimInstance` (`self.Mesh`)) (`local.SectionName`) _attackmontage)
      (`/Engine/EditorBlueprintResources/StandardMacros.IsValid` _sfx
        (:`Is Valid`
          (`GameplayStatics.PlaySoundAtLocation` _sfx (`self.K2_GetActorLocation`) (struct) 1.0 1.0 0.0 null null null null))
        (:`Is Not Valid`
          _))
      (`KismetSystemLibrary.K2_SetTimer` null "EndAttack" 1.5)
      (`KismetSystemLibrary.K2_SetTimer` null "ResetAttackCooldown" (`self.AttackCooldown`)))
    (:`else`)))

(fn `ResetAttackCooldown`
  (set `self.bCanAttack` true))

(fn `ResetDashCooldown`
  (set `self.bCanDash` true))

(fn `ResetHitReact`
  (set `self.bCanReactToHit` true))

(fn `TurnOnRagdoll`
  (`PrimitiveComponent.SetSimulatePhysics` (`self.Mesh`) true)
  (`PrimitiveComponent.SetSimulatePhysics` (`self.R_Arm`) true)
  (`PrimitiveComponent.SetSimulatePhysics` (`self.Lower_Torso`) true)
  (`PrimitiveComponent.SetSimulatePhysics` (`self.L_Leg`) true)
  (`PrimitiveComponent.SetSimulatePhysics` (`self.L_Arm`) true)
  (`PrimitiveComponent.SetSimulatePhysics` (`self.Head`) true)
  (`PrimitiveComponent.SetSimulatePhysics` (`self.R_Leg`) true))

(fn `UserConstructionScript`
  (`SkinnedMeshComponent.SetLeaderPoseComponent` (`self.L_Arm`) (`self.Mesh`) false false)
  (`SkinnedMeshComponent.SetLeaderPoseComponent` (`self.L_Leg`) (`self.Mesh`) false false)
  (`SkinnedMeshComponent.SetLeaderPoseComponent` (`self.Lower_Torso`) (`self.Mesh`) false false)
  (`SkinnedMeshComponent.SetLeaderPoseComponent` (`self.R_Arm`) (`self.Mesh`) false false)
  (`SkinnedMeshComponent.SetLeaderPoseComponent` (`self.R_Leg`) (`self.Mesh`) false false)
  (`SkinnedMeshComponent.SetLeaderPoseComponent` (`self.Head`) (`self.Mesh`) false false))