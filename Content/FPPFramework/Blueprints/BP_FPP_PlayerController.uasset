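; First-person framework player controller that manages input setup, the HUD and the death screen for the local player.
; On possess it enables pawn input, switches to game-only input, adds the default Enhanced Input mapping context and shows the HUD widget.
; CreateDeathScreen disables pawn input, removes the HUD, shows the death screen widget in UI-only input mode and reveals the mouse cursor.
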(event `self.ReceivePossess`
  (params (PossessedPawn :type "Pawn Object Reference"))
  (`self.EnableInput` (`self.K2_GetPawn`) self)
  (`WidgetBlueprintLibrary.SetInputMode_GameOnly` self)
  (`self.SetupInput`)
  (`self.SetupHUD`))

(fn `CreateDeathScreen`
  (`self.DisableInput` (`self.K2_GetPawn`) self)
  (bind _hud_widget (`self.HUD_Widget`)
    (:`then`
      (`Widget.RemoveFromParent` _hud_widget))
    (:`else`
      _))
  (bind _returnvalue (`|CreateWidget` "/Game/FPPFramework/Widgets/DeathScreen/WBP_DeathScreen.WBP_DeathScreen_C"))
  (`UserWidget.AddToViewport` _returnvalue 0)
  (`WidgetBlueprintLibrary.SetInputMode_UIOnlyEx` self _returnvalue)
  (set `self.bShowMouseCursor` true))

(fn `SetupHUD`
  (bind _returnvalue (`|CreateWidget` "/Game/FPPFramework/Widgets/WBP_HUD.WBP_HUD_C"))
  (bind _output_get (set `self.HUD_Widget` _returnvalue))
  (`UserWidget.AddToViewport` _output_get 0))

(fn `SetupInput`
  (`EnhancedInputSubsystemInterface.AddMappingContext` (subsystem `EnhancedInputLocalPlayerSubsystem`) "/Game/FPPFramework/Input/IMC_Default.IMC_Default" 0 (struct)))

(fn `UserConstructionScript`)